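; Interactable door that swings open and closed with a creak, optionally requiring a named key in the first-person character's inventory.
; Interact toggles IsOpen and plays or reverses a timeline driving door yaw; only keyless doors ignore interaction mid-swing.
; A missing key plays a locked sound, throttled by a DoOnce reset after a delay.
; GetInteractPrompt reports "Locked" for any key door, otherwise open/close text; an older DoorRotation timeline remains unconnected.
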(event `/Game/BluePrints/BPI_Interactable.Interact`
  (params (Caller :type "/Game/FirstPerson/Blueprints/BP_FirstPersonCharacter Object Reference"))
  (if (`self.bRequiresKey`)
    (bind _asbp_first_person_character (cast `/Game/FirstPerson/Blueprints/BP_FirstPersonCharacter` Caller))
    (if (`KismetArrayLibrary.Array_Contains` (`/Game/FirstPerson/Blueprints/BP_FirstPersonCharacter.Inventory` _asbp_first_person_character) (`self.RequiredKeyName`))
      (`GameplayStatics.PlaySoundAtLocation` "/Game/FreeSound/455324__rambler52__heavy-door-creaking_05.455324__rambler52__heavy-door-creaking_05" (0.0 0.0 0.0) (struct) 1.0 1.0 0.0 null null null null :!label _label)
      (bind _output_get (set `self.IsOpen` (not (`self.IsOpen`))))
      (if _output_get
        (bind (_direction _alpha) (`Timeline|타임라인` :!label _label_2)
          (:`Update`
            (`SceneComponent.K2_SetRelativeRotation` (`self.Door`) (`KismetMathLibrary.MakeRotator` 0.0 0.0 _alpha) false false)))
        (else
          (goto _label_2 :!via `Reverse`)))
      (else
        (`/Engine/EditorBlueprintResources/StandardMacros.DoOnce` false :!label _label_3
          (:`Completed`
            (`GameplayStatics.PlaySoundAtLocation` "/Game/FreeSound/391724__jpolito__jp_circuitbox_locked01.391724__jpolito__jp_circuitbox_locked01" (0.0 0.0 0.0) (struct) 1.0 1.0 0.0 null null null null)
            (`KismetSystemLibrary.Delay` 0.8)
            (goto _label_3 :!via `Reset`)))))
    (elif (not (`TimelineComponent.IsPlaying` (`self.타임라인`)))
      (goto _label))))

(fn `GetInteractPrompt`
  (returns (`Open Door` :type Text))
  (if (`self.bRequiresKey`)
    (return "Locked")
    (else
      (return (select `bool` (`self.IsOpen`) :`false` "OpenDoor" :`true` "Close Door" :!type "Text")))))

(fn `UserConstructionScript`)